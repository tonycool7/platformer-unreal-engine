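; Bat enemy, derived from a parent enemy class, that moves continuously along the world X axis.
; BeginPlay randomly sets MoveLeft, and Tick uses it to feed positive or negative movement input, with no logic to change direction afterward.
; Its death handler runs the parent's EnemyDied and then destroys the actor.
; Actor overlap only prints a placeholder debug string.
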(event EventBeginPlay
  (Variables|Default|SetMoveLeft (Math|Random|RandomBool)))

(event Collision|EventActorBeginOverlap
  (params (OtherActor :type Actor%20Object%20Reference))
  (Development|PrintString "Hello"))

(event EventTick
  (params (DeltaSeconds :type Float%20%28single-precision%29))
  (Pawn|Input|AddMovementInput "1.000000, 0, 0" (Math|Float|SelectFloat 1.0 -1.0 (Variables|Default|GetMoveLeft)) false))

(fn ConstructionScript
  (|CallParentFunction))

(fn EnemyDied
  (|CallParentFunction)
  (Actor|DestroyActor))